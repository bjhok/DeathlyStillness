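; Player character Blueprint that drives jump, crouch and gun-holding states on its ABP_PlayerAnim instance, cached at BeginPlay.
; SetJumpAnim plays a walk, jog or run jump montage by movement State, then re-enables jumping after a delay.
; SetCrouchVal forwards crouch state to the anim instance.
; Key 1 toggles the gun anim flags and plays or reverses a timeline that slides the spring arm's lateral socket offset.
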(event EventBeginPlay
  (bind _asabp_player_anim_1 (Utilities|Casting|CastToABP_PlayerAnim (Components|SkeletalMesh|GetAnimInstance (Variables|Character|GetMesh))))
  (Variables|Default|SetAs%20ABP%20Player%20Anim _asabp_player_anim_1))

(event Collision|EventActorBeginOverlap
  (params (OtherActor :type Actor%20Object%20Reference)))

(event EventTick
  (params (DeltaSeconds :type Float%20%28single-precision%29)))

(event EventSetJumpAnim
  (Variables|/Script/DeathlyStillness.DSPlayerAnim|SetIsJump (Variables|Default|GetAs%20ABP%20Player%20Anim) true)
  (CallFunction|设置跳跃动画 "/Game/Character/ActionPak/Mobility_01/Animation/Root_Motion/Jump/MOB1_M1_Walk_F_Jump_RU_Montage.MOB1_M1_Walk_F_Jump_RU_Montage" "/Game/Character/ActionPak/Mobility_01/Animation/Root_Motion/Jump/MOB1_M1_Jog_F_Jump_RU_Montage.MOB1_M1_Jog_F_Jump_RU_Montage" "/Game/Character/ActionPak/Mobility_01/Animation/Root_Motion/Jump/MOB1_M1_Run_F_Jump_RU_Montage.MOB1_M1_Run_F_Jump_RU_Montage")
  (Utilities|FlowControl|Delay 1.0)
  (Variables|Default|SetPlayerCanJump true)
  (Variables|/Script/DeathlyStillness.DSPlayerAnim|SetIsJump (Variables|Default|GetAs%20ABP%20Player%20Anim) false))

(event EventSetCrouchVal
  (params (CanCrouch :type Boolean))
  (Variables|/Script/DeathlyStillness.DSPlayerAnim|SetIsCrouch (Variables|Default|GetAs%20ABP%20Player%20Anim) CanCrouch))

(event Input|KeyboardEvents|1
  (params (Key :type Key%20Structure :default "None"))
  (bind _as_abp_player_anim (Variables|Default|GetAs%20ABP%20Player%20Anim))
  (bind _springarmcomp (Variables|Default|GetSpringArmComp))
  (:Pressed
    (if (Variables|/Script/DeathlyStillness.DSPlayerAnim|GetIsHoldGun _as_abp_player_anim)
      (Variables|/Script/DeathlyStillness.DSPlayerAnim|SetIsHoldGun _as_abp_player_anim false)
      (Variables|/Script/DeathlyStillness.DSPlayerAnim|SetEquipWeaponDir _as_abp_player_anim -1.0)
      (Variables|/Script/DeathlyStillness.DSPlayerAnim|SetIsEquipWeapon _as_abp_player_anim false)
      (bind _新建轨道_0 (Timeline|HaveGunSwitch Reverse)
        (:Update
          (Variables|/Script/Engine.SpringArmComponent|SetSocketOffset _springarmcomp (Math|Vector|MakeVector 0.0 (Math|Float|Lerp 15.0 -35.0 _新建轨道_0) (.z (Variables|/Script/Engine.SpringArmComponent|GetSocketOffset _springarmcomp))))))
      (else
        (Variables|/Script/DeathlyStillness.DSPlayerAnim|SetIsHoldGun _as_abp_player_anim true)
        (Variables|/Script/DeathlyStillness.DSPlayerAnim|SetEquipWeaponDir _as_abp_player_anim 1.0)
        (Variables|/Script/DeathlyStillness.DSPlayerAnim|SetIsEquipWeapon _as_abp_player_anim true)
        (Timeline|HaveGunSwitch Play)))))

(fn ConstructionScript)

(fn 设置跳跃动画
  (params (WalkJumpAnim :type Anim%20Montage%20Object%20Reference) (JogJumpAnim :type Anim%20Montage%20Object%20Reference) (RunJumpAnim :type Anim%20Montage%20Object%20Reference))
  (switch Utilities|FlowControl|Switch|SwitchonEPlayerState (Variables|Default|GetState)
    (:Walk
      (Variables|Default|SetJumpAnim WalkJumpAnim))
    (:Jog
      (Variables|Default|SetJumpAnim JogJumpAnim))
    (:Run
      (Variables|Default|SetJumpAnim RunJumpAnim)))
  (Animation|Montage|MontagePlay (Components|SkeletalMesh|GetAnimInstance (Variables|Character|GetMesh)) (Variables|Default|GetJumpAnim) 1.0 "MontageLength" 0.0 true))